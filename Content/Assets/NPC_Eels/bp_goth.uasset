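; Goth NPC actor that shows a room-specific dialogue and flaps its mouth while talking.
; When the player character's Head-tagged component overlaps its Box, a DoOnce creates the widget selected by RoomNumber, registers the NPC as speaker through IDialogue and loops into a timeline-driven Mouth rotation.
; EndDialogue stops the mouth, while ResetActor re-arms the DoOnce and removes the widget.
; Older per-room branches remain, largely disconnected.
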(event OnComponentBeginOverlap(Box)
  (params (OverlappedComponent :type Primitive%20Component%20Object%20Reference) (OtherActor :type Actor%20Object%20Reference) (OtherComp :type Primitive%20Component%20Object%20Reference) (OtherBodyIndex :type Integer) (bFromSweep :type Boolean) (SweepResult :type Hit%20Result%20Structure%20%28by%20ref%29))
  (bind _doesit (CallFunction|ComponentHasTag OtherComp "Head"))
  (if _doesit
    (Utilities|Casting|CastToBP_ThirdPersonCharacter OtherActor)
    (Utilities|FlowControl|DoOnce false
      (:Completed
        (bind _returnvalue (UserInterface|CreateWidget (Utilities|Select :Index (Variables|Default|GetRoomNumber) :Option%200 "/Game/Widgets/Dialogue/w_dialogue_office.w_dialogue_office_C" :Option%201 "/Game/Widgets/Dialogue/w_dialogue_hallway.w_dialogue_hallway_C" :Option%202 "/Game/Widgets/Dialogue/w_dialogue_grates.w_dialogue_grates_C" :Option%203 "/Game/Widgets/Dialogue/w_dialogue_factory.w_dialogue_factory_C") (Game|GetPlayerController 0)))
        (bind _asidialogue (Utilities|Casting|CastToIDialogue _returnvalue)
          (:then
            (Default|AddSpeaker _asidialogue self))
          (:CastFailed
            _))
        (bind _output_get (Variables|Default|SetCurrentDialogueWidget _returnvalue))
        (UserInterface|Viewport|AddtoViewport _output_get 0)
        (bind _rotate (Timeline|Rotate Play)
          (:Update
            (Transformation|SetRelativeRotation (Variables|Default|Getmouth) (Math|Rotator|MakeRotator (Math|Float|Lerp -47.0 2e+01 _rotate) 0.0 0.0) false false)))))))

(event Custom|Reset%20Room%201
  (Utilities|FlowControl|DoOnce false) ; enters at Reset
)

(event Custom|Reset%20Room%202
  (Utilities|FlowControl|DoOnce false) ; enters at Reset
)

(event Custom|Reset%20Room
  (Utilities|FlowControl|DoOnce false) ; enters at Reset
)

(event Custom|Reset%20Room%203
  (Utilities|FlowControl|DoOnce false) ; enters at Reset
)

(event Custom|Reset%20Room%204
  (Utilities|FlowControl|DoOnce false) ; enters at Reset
)

(event EventResetActor
  (CallFunction|ResetRoom)
  (Widget|RemovefromParent (Variables|Default|GetCurrentDialogueWidget)))

(event EventEndDialogue
  (Transformation|SetRelativeRotation (Variables|Default|Getmouth) "0.000000,0.000000,-47.000000" false false)
  (bind _rotate (Timeline|Rotate Stop)
    (:Update
      (Transformation|SetRelativeRotation (Variables|Default|Getmouth) (Math|Rotator|MakeRotator (Math|Float|Lerp -47.0 2e+01 _rotate) 0.0 0.0) false false))))

(fn ConstructionScript)