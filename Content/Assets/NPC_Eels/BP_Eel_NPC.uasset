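; Eel NPC that starts a one-time dialogue when a "Head"-tagged component of the player character overlaps its spawn collider.
; RoomNumber selects the dialogue widget and voice sound, and the eel registers as speaker through IDialogue.
; A timeline animates the jaw hinge until EndDialogue stops the sound and closes the mouth.
; ResetActor re-arms the trigger and removes the current widget.
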(event OnComponentBeginOverlap(DialogueSpawnCollider)
  (params (OverlappedComponent :type Primitive%20Component%20Object%20Reference) (OtherActor :type Actor%20Object%20Reference) (OtherComp :type Primitive%20Component%20Object%20Reference) (OtherBodyIndex :type Integer) (bFromSweep :type Boolean) (SweepResult :type Hit%20Result%20Structure%20%28by%20ref%29))
  (bind _doesit (CallFunction|ComponentHasTag OtherComp "Head"))
  (if _doesit
    (Utilities|Casting|CastToBP_ThirdPersonCharacter OtherActor)
    (Utilities|FlowControl|DoOnce false
      (:Completed
        (bind _returnvalue (UserInterface|CreateWidget (Utilities|Select :Index (Variables|Default|GetRoomNumber) :Option%200 0 :Option%201 "/Game/Widgets/Dialogue/w_dialogue_office.w_dialogue_office_C" :Option%202 "/Game/Widgets/Dialogue/w_dialogue_hallway.w_dialogue_hallway_C" :Option%203 "/Game/Widgets/Dialogue/w_dialogue_grates.w_dialogue_grates_C" :Option%204 "/Game/Widgets/Dialogue/w_dialogue_factory.w_dialogue_factory_C") (Game|GetPlayerController 0)))
        (bind _asidialogue (Utilities|Casting|CastToIDialogue _returnvalue)
          (:then
            (Default|AddSpeaker _asidialogue self)
            (CallFunction|StartDialogueSound))
          (:CastFailed
            _))
        (bind _output_get (Variables|Default|SetCurrentDialogueWidget _returnvalue))
        (UserInterface|Viewport|AddtoViewport _output_get 0)
        (bind _alpha (Timeline|Rotate%20Jaw Play)
          (:Update
            (Transformation|SetRelativeRotation (Variables|Default|GetJawHinge) (Math|Rotator|Lerp(Rotator) (Variables|Default|GetClosedJawRotation) (Variables|Default|GetOpenJawRotation) _alpha true) false false)))))))

(event Custom|Reset%20Dialogue
  (Utilities|FlowControl|DoOnce false) ; enters at Reset
)

(event Custom|Start%20Dialogue%20Sound
  (bind _returnvalue (Audio|SpawnSoundatLocation (Utilities|Select :Index (Variables|Default|GetRoomNumber) :Option%200 0 :Option%201 "/Game/Audio/Meta_Sounds/ms_Eel_1.ms_Eel_1" :Option%202 "/Game/Audio/Meta_Sounds/ms_Eel_2.ms_Eel_2" :Option%203 "/Game/Audio/Meta_Sounds/ms_Eel_3.ms_Eel_3" :Option%204 "/Game/Audio/Meta_Sounds/ms_Eel_4.ms_Eel_4") (Transformation|GetWorldLocation (Variables|Default|GetJawHinge)) "0, 0, 0" 1.0 1.0 0.0 0 0)))

(event Custom|Stop%20Dialogue%20Sound
  (Utilities|IsValid (stale Custom|Start%20Dialogue%20Sound _returnvalue)
    (:Is%20Valid
      (Audio|Components|Audio|Stop (stale Custom|Start%20Dialogue%20Sound _returnvalue))
      (Components|DestroyComponent (stale Custom|Start%20Dialogue%20Sound _returnvalue)))))

(event EventBeginPlay)

(event Collision|EventActorBeginOverlap
  (params (OtherActor :type Actor%20Object%20Reference)))

(event EventTick
  (params (DeltaSeconds :type Float%20%28single-precision%29)))

(event EventResetActor
  (bind _currentdialoguewidget (Variables|Default|GetCurrentDialogueWidget))
  ;[1 1 1] Reset Actor
  (CallFunction|ResetDialogue)
  (Utilities|IsValid _currentdialoguewidget
    (:Is%20Valid
      (Widget|RemovefromParent _currentdialoguewidget))))

(event EventEndDialogue
  ;[1 1 1] End Dialogue
  (CallFunction|StopDialogueSound)
  (Transformation|SetRelativeRotation (Variables|Default|GetJawHinge) (Variables|Default|GetClosedJawRotation) false false)
  (bind _alpha (Timeline|Rotate%20Jaw Stop)
    (:Update
      (Transformation|SetRelativeRotation (Variables|Default|GetJawHinge) (Math|Rotator|Lerp(Rotator) (Variables|Default|GetClosedJawRotation) (Variables|Default|GetOpenJawRotation) _alpha true) false false))))

(fn ConstructionScript)