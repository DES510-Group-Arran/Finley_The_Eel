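; BP_Fade is a red magical wall whose material fades when the capsule overlap events fire.
; BeginPlay creates a dynamic material instance on the Cube and initializes its Fade Amount parameter.
; CapsuleOverlapStart plays the FadeInOut timeline to drive that parameter, and CapsuleOverlapEnd reverses it.
; The Box overlap handlers are empty, and nothing in the graph calls the capsule events.
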(event OnComponentBeginOverlap(Box)
  (params (OverlappedComponent :type Primitive%20Component%20Object%20Reference) (OtherActor :type Actor%20Object%20Reference) (OtherComp :type Primitive%20Component%20Object%20Reference) (OtherBodyIndex :type Integer) (bFromSweep :type Boolean) (SweepResult :type Hit%20Result%20Structure%20%28by%20ref%29)))

(event OnComponentEndOverlap(Box)
  (params (OverlappedComponent :type Primitive%20Component%20Object%20Reference) (OtherActor :type Actor%20Object%20Reference) (OtherComp :type Primitive%20Component%20Object%20Reference) (OtherBodyIndex :type Integer)))

(event EventBeginPlay
  (bind _returnvalue (Rendering|Material|CreateDynamicMaterialInstance (Variables|Default|GetCube) 0 "/Game/Materials/Magical_Walls/m_magical_wall_red.m_magical_wall_red" "None" :!class /Script/Engine.PrimitiveComponent))
  (bind _output_get (Variables|Default|SetDynamic%20Variable _returnvalue))
  (Rendering|Material|SetScalarParameterValue _output_get "Fade Amount" -1.0 :!class /Script/Engine.MaterialInstanceDynamic))

(event EventCapsuleOverlapStart
  (Components|Timeline|SetPlayRate (Variables|Default|GetFade%20In/Out) 0.9)
  (bind _newtrack_0 (Timeline|Fade%20In/Out Play)
    (:Update
      (Rendering|Material|SetScalarParameterValue (Variables|Default|GetDynamic%20Variable) "Fade Amount" _newtrack_0 :!class /Script/Engine.MaterialInstanceDynamic))))

(event EventCapsuleOverlapEnd
  (bind _newtrack_0 (Timeline|Fade%20In/Out Reverse)
    (:Update
      (Rendering|Material|SetScalarParameterValue (Variables|Default|GetDynamic%20Variable) "Fade Amount" _newtrack_0 :!class /Script/Engine.MaterialInstanceDynamic))))

(fn ConstructionScript)