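; Resettable physics object Blueprint for static level props, built around a single Obj component.
; BeginPlay caches Obj's relative transform, and the ResetActor event teleports it back to that transform without sweeping.
; Any begin overlap on Obj plays the Ms_water_charge sound at its world location, with no filter on the overlapping actor.
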(event OnComponentBeginOverlap(Obj)
  (params (OverlappedComponent :type Primitive%20Component%20Object%20Reference) (OtherActor :type Actor%20Object%20Reference) (OtherComp :type Primitive%20Component%20Object%20Reference) (OtherBodyIndex :type Integer) (bFromSweep :type Boolean) (SweepResult :type Hit%20Result%20Structure%20%28by%20ref%29))
  (Audio|PlaySoundatLocation "/Game/Audio/Meta_Sounds/ms_water_charge.ms_water_charge" (Transformation|GetWorldLocation (Variables|Default|GetObj)) "0, 0, 0" 1.0 1.0 0.0 0 0 0 0))

(event EventBeginPlay
  (Variables|Default|SetIntitial%20Transform (Transformation|GetRelativeTransform (Variables|Default|GetObj))))

(event EventResetActor
  (Transformation|SetRelativeTransform (Variables|Default|GetObj) (Variables|Default|GetIntitial%20Transform) false true))

(fn ConstructionScript)